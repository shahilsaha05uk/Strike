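; Level 1 game mode that tracks joining player controllers and creates team-based spawn points.
; When a new player starts, it runs the parent logic, then adds controllers implementing ControllerInterface to a unique Controllers list, whose RepNotify is empty.
; SpawnPlayerStart looks up a team in the TeamBases map and spawns a PlayerStart at a random XY inside that base's box, at a fixed height.
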(event `self.HandleStartingNewPlayer`
  (params (NewPlayer :type "PlayerController Object Reference"))
  (`parent.HandleStartingNewPlayer` NewPlayer)
  (if (`KismetSystemLibrary.DoesImplementInterface` NewPlayer "/Script/MultiplayerProject.ControllerInterface")
    (`KismetArrayLibrary.Array_AddUnique` (`self.Controllers`) NewPlayer)))

(fn `OnRep_Controllers`)

(fn `SpawnPlayerStart`
  (params (Team :type "ETeam Enum" :default "NONE"))
  (returns (Value :type "PlayerStart Object Reference"))
  (bind _keys (`BlueprintMapLibrary.Map_Keys` (`self.TeamBases`)))
  (bind _returnvalue (`KismetArrayLibrary.Array_Find` _keys Team))
  (if (!= _returnvalue -1)
    (bind _values (`BlueprintMapLibrary.Map_Values` (`self.TeamBases`)))
    (bind (_origin _boxextent) (`KismetSystemLibrary.GetComponentBounds` (`/Game/TEST_AND_DEBUG/BP_LocVolume.Box` (`|GetArrayItem` _values _returnvalue))))
    (bind (_returnvalue_x _returnvalue_y) (`KismetMathLibrary.BreakVector` (`KismetMathLibrary.RandomPointInBoundingBox` _origin _boxextent)))
    (bind _returnvalue_2 (`|SpawnActorFromClass` "/Script/Engine.PlayerStart" (`KismetMathLibrary.MakeTransform` (`KismetMathLibrary.MakeVector` _returnvalue_x _returnvalue_y 5.0)) "Undefined" "MultiplyWithRoot" null null))
    (return _returnvalue_2)))

(fn `UserConstructionScript`)