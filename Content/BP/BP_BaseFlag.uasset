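; BP_BaseFlag is a base flag actor that can be captured and returned to its starting spot.
; It stores the flag mesh's world transform at BeginPlay, and capture attaches the mesh to a supplied component socket.
; A capture call while already captured instead calls RetrieveFlag and clears the captured state.
; The retrieved event reattaches the mesh to its parent component and restores the stored transform.
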(event `self.OnFlagCaptured`
  (params (MeshToAttachTo :type "SkeletalMeshComponent Object Reference") (SocketName :type Name))
  (bind _mflag (`self.mFlag`))
  (if (`self.bIsCaptured`)
    (`FlagInterface.RetrieveFlag`)
    (set `self.bIsCaptured` false)
    (else
      (`KismetSystemLibrary.PrintString` "Flag has been Captured")
      (`SceneComponent.K2_DetachFromComponent` _mflag "KeepWorld" "KeepWorld" "KeepWorld" true)
      (`SceneComponent.K2_AttachToComponent` _mflag MeshToAttachTo SocketName "SnapToTarget" "SnapToTarget" "KeepRelative" true)
      (set `self.bIsCaptured` true))))

(event `self.ReceiveBeginPlay`
  (set `self.InitialTransform` (`SceneComponent.K2_GetComponentToWorld` (`self.mFlag`))))

(event `self.OnFlagRetrieved`
  (bind _mflag (`self.mFlag`))
  (`KismetSystemLibrary.PrintString` "Flag has been Retrieved")
  (`SceneComponent.K2_DetachFromComponent` _mflag "KeepWorld" "KeepWorld" "KeepWorld" true)
  (`SceneComponent.K2_AttachToComponent` _mflag (`self.mFlagParent`) "None" "KeepWorld" "KeepWorld" "KeepRelative" true)
  (`SceneComponent.K2_SetWorldTransform` (`self.mFlag`) (`self.InitialTransform`) false false))

(fn `UserConstructionScript`)