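; BP_FlagBase is a base flag actor that can be captured onto a mesh socket and returned to its starting spot.
; It stores the flag component's world transform on BeginPlay.
; OnFlagCaptured snaps the flag to the given mesh socket, or calls RetrieveFlag if it is already captured.
; RetrieveFlag reattaches the flag to the root and restores the stored transform.
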(event `self.ReceiveBeginPlay`
  (set `self.InitialPosition` (`SceneComponent.K2_GetComponentToWorld` (`self.mFlagComponent`))))

(event `self.OnFlagCaptured`
  (params (MeshToAttachTo :type "SkeletalMeshComponent Object Reference") (SocketName :type Name))
  (bind _mflagcomponent (`self.mFlagComponent`))
  (if (`self.bIsCaptured`)
    (`FlagInterface.RetrieveFlag`)
    (set `self.bIsCaptured` false)
    (else
      (`KismetSystemLibrary.PrintString` "Flag has been Captured")
      (`SceneComponent.K2_DetachFromComponent` _mflagcomponent "KeepWorld" "KeepWorld" "KeepWorld" true)
      (`SceneComponent.K2_AttachToComponent` _mflagcomponent MeshToAttachTo SocketName "SnapToTarget" "SnapToTarget" "KeepRelative" true)
      (set `self.bIsCaptured` true))))

(event `FlagInterface.RetrieveFlag`
  (bind _mflagcomponent (`self.mFlagComponent`))
  (`KismetSystemLibrary.PrintString` "Flag has been Retrieved")
  (`SceneComponent.K2_DetachFromComponent` _mflagcomponent "KeepWorld" "KeepWorld" "KeepWorld" true)
  (`SceneComponent.K2_AttachToComponent` _mflagcomponent (`self.mRoot`) "None" "KeepWorld" "KeepWorld" "KeepRelative" true)
  (`SceneComponent.K2_SetWorldTransform` (`self.mFlagComponent`) (`self.InitialPosition`) false false))

(fn `UserConstructionScript`)