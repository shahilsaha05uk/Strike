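; Base multiplayer player character Blueprint for a team game with weapons and a flag.
; Aim start and stop route through server RPCs to multicasts that call parent logic, and other multicasts handle flag drops and health bar updates.
; The local client sends its GameInstance username to the server, while OnRep functions push name and team to the overhead widget, retrying on timers until it exists.
; Death handling and camera aim moves are left disconnected.
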(event `PlayerInputInterface.StartAiming`
  ;[0 0 0] On Aiming
  (`self.ServerRPC_AimStart`))

(event `ServerRPC_AimStart`
  ;[0 0 0] On Aiming
  (`self.MulticastRPC_AimStart`))

(event `MulticastRPC_AimStart`
  ;[0 0 0] On Aiming
  (`parent.StartAiming`))

(event `PlayerInputInterface.StopAiming`
  ;[0 0 0] On Aiming
  (`self.ServerRPC_StopAim`))

(event `ServerRPC_StopAim`
  ;[0 0 0] On Aiming
  (`self.MulticastRPC_StopAim`))

(event `MulticastRPC_StopAim`
  ;[0 0 0] On Aiming
  (`parent.StopAiming`))

(event `self.BlueprintMulticast_DropFlag`
  (message `FlagInterface.OnDropped` (`self.mFlagRef`)))

(event `self.BlueprintMulticast_UpdateHealthBar`
  (params (Health :type "Float (single-precision)"))
  (`/Game/UI/W_PlayerOverheadUI.UpdateHealth` (`self.OverheadUI`) Health))

(event `self.ReceivePossessed`
  (params (NewController :type "Controller Object Reference"))
  (bind _returnvalue (message `PlayerStateInterface.GetPlayerDetails` (`self.PlayerState`)))
  (bind _output_get (set `self.PlayerDetails` _returnvalue))
  (bind (_playername _currentmoney _team) (break `PlayerDetails` _output_get))
  (`KismetSystemLibrary.PrintString` (`KismetStringLibrary.Concat_StrStr` "Team: " (`|GetEnumeratorNameAsString` _team) ", Money: " (`KismetStringLibrary.Conv_IntToString` _currentmoney)) true true (struct :`A` 1.0) 20.0))

(event `Client_SetPlayerName`
  ;[0 0 0 1 15] Solution To Updating the Player Name
  (if (`self.IsLocallyControlled`)
    (bind _asbp_multiplayer_game_instance (cast `/Game/BP_MultiplayerGameInstance` (`GameplayStatics.GetGameInstance`)))
    (`self.Server_SetPlayerName` (`/Game/BP_MultiplayerGameInstance.Username` _asbp_multiplayer_game_instance))))

(event `Server_SetPlayerName`
  (params (UserName :type Text))
  ;[0 0 0 1 15] Solution To Updating the Player Name
  (set `self.UserName` UserName))

(event `self.BlueprintMulticast_OnDead`
  (params (InstigatedBy :type "Controller Object Reference")))

(event `self.BlueprintServer_SpawnWeapon`
  (params (Weapon :type "BaseWeapon Object Reference"))
  (bind _asbp_base_weapon (cast `/Game/BP/BP_BaseWeapon` Weapon))
  (set `/Game/BP/BP_BaseWeapon.IsPickedUp` true _asbp_base_weapon))

(fn `OnRep_PlayerDetails`
  (bind ((`PlayerName` _playername) (`Team` _team)) (break `PlayerDetails` (`self.PlayerDetails`)))
  (bind _returnvalue (`WidgetComponent.GetWidget` (`self.PlayerTagWidget`)))
  (`/Engine/EditorBlueprintResources/StandardMacros.IsValid` _returnvalue
    (:`Is Valid`
      (bind _asw_player_overhead_ui (cast `/Game/UI/W_PlayerOverheadUI` _returnvalue))
      (bind _output_get (set `self.OverheadUI` _asw_player_overhead_ui))
      (`/Game/UI/W_PlayerOverheadUI.UpdateTeam` _output_get _team _playername)
      (`SceneComponent.SetHiddenInGame` (`self.PlayerTagWidget`) false false))
    (:`Is Not Valid`
      (`KismetSystemLibrary.K2_SetTimer` null "OnRep_PlayerDetails" 0.1))))

(fn `OnRep_UserName`
  (bind _returnvalue (`WidgetComponent.GetWidget` (`self.PlayerTagWidget`)))
  (`/Engine/EditorBlueprintResources/StandardMacros.IsValid` _returnvalue
    (:`Is Valid`
      (bind _asw_player_overhead_ui (cast `/Game/UI/W_PlayerOverheadUI` _returnvalue))
      (`/Game/UI/W_PlayerOverheadUI.UpdateName` _asw_player_overhead_ui (`self.UserName`)))
    (:`Is Not Valid`
      (`KismetSystemLibrary.K2_SetTimer` null "OnRep_UserName" 0.2))))

(fn `SetHealth`
  (params (Value :type "Float (single-precision)")))

(fn `SetMesh`
  (locals (M1 :type "SkeletalMesh Object Reference" :default "/Script/Engine.SkeletalMesh'/Game/__ExternalAssets/Elite_Soldiers/Mesh/Full_Mesh/SK_Elite_Soldier_Full_03.SK_Elite_Soldier_Full_03'") (M2 :type "SkeletalMesh Object Reference" :default "/Script/Engine.SkeletalMesh'/Game/__ExternalAssets/Elite_Soldiers/Mesh_UE5/Full/SKM_Elite_Soldier_Full_04.SKM_Elite_Soldier_Full_04'"))
  (if (== (`SkeletalMeshComponent.GetSkeletalMeshAsset` (`self.Mesh`)) (`local.M1`))
    (`SkeletalMeshComponent.SetSkeletalMeshAsset` (`self.Mesh`) (`local.M2`))
    (else
      (`SkeletalMeshComponent.SetSkeletalMeshAsset` (`self.Mesh`) (`local.M1`)))))

(fn `UserConstructionScript`)