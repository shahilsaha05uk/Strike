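; Multiplayer player character Blueprint with an overhead-style UI widget, socketed weapon, flag capture and focused-actor tracking.
; Possession refreshes the controller UI, the PlayerDetails RepNotify updates the widget, and a multicast event either destroys the held weapon or spawns and attaches one.
; Flag capture passes the mesh socket through an interface; pickup and death are unfinished stubs.
; A debug key tests server-to-multicast calls by swapping meshes.
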(event `Update UI`
  (params (InputPin :type "PlayerDetails Structure"))
  ;[0 0 0] Update Overlay UI
  (bind _asplayer_ui (cast `/Game/UI/PlayerUI` (`WidgetComponent.GetWidget` (`self.mOverlayWidget`))))
  (`/Game/UI/PlayerUI.UpdateVals` _asplayer_ui InputPin))

(event `self.BlueprintMulticast_SpawnWeapon`
  (params (WeaponDetails :type "WeaponDetails Structure"))
  ;[0 0 0] Spawn Weapon
  (bind _returnvalue (`self.GetWeapon`))
  (`/Engine/EditorBlueprintResources/StandardMacros.IsValid` _returnvalue
    (:`Is Valid`
      (`self.K2_DestroyActor` _returnvalue))
    (:`Is Not Valid`
      (bind _returnvalue_2 (`|SpawnActorFromClass` (`.WeaponAsset` (break `WeaponDetails` WeaponDetails)) (`self.GetTransform`) "Undefined" "MultiplyWithRoot" null null))
      (`self.SetWeapon` _returnvalue_2)
      (bind _returnvalue_3 (`self.GetWeapon`))
      (`self.K2_AttachToComponent` _returnvalue_3 (`self.Mesh`) (`self.WeaponSocket`) "SnapToTarget" "SnapToTarget" "KeepRelative" true))))

(event `self.ReceivePossessed`
  (params (NewController :type "Controller Object Reference"))
  (bind _asbp_controller (cast `/Game/BP_Controller` NewController))
  (`/Game/BP_Controller.IA_RefreshUI` _asbp_controller))

(event `self.Collect`
  (bind _returnvalue (`self.GetFocusedActorDetails`))
  (if (`KismetSystemLibrary.DoesImplementInterface` (`.ActorReference` (break `FocusedActorDetails` _returnvalue)) "/Script/MultiplayerProject.PickupInterface")
    _))

(event `self.CaptureFlag`
  (bind _returnvalue (`self.GetFocusedActorDetails`))
  (bind (_actorname _interacttype _actorreference) (break `FocusedActorDetails` _returnvalue))
  (if (`KismetSystemLibrary.DoesImplementInterface` _actorreference "/Script/MultiplayerProject.FlagInterface")
    (bind _output_get (set `self.FlagRef` _actorreference))
    (message `FlagInterface.CaptureFlag` _output_get (`self.Mesh`) (`self.FlagSocket`))))

(event `Key|L`
  (params (Key :type "Key Structure"))
  (:`Released`
    (`self.OnDead`)))

(event `OnDead`
  (`KismetSystemLibrary.PrintString` "Player Died")
  (`/Engine/EditorBlueprintResources/StandardMacros.IsValid` (`self.FlagRef`)
    (:`Is Valid`
      (`KismetSystemLibrary.PrintString` "Need to Drop the Flag"))
    (:`Is Not Valid`
      (`KismetSystemLibrary.PrintString` "No Flags Found on the player"))))

(event `InputsInterface.UpdateFocusedActor`
  (params (Details :type "FocusedActorDetails Structure"))
  (`self.SetFocusedActorDetails` Details)
  (bind _returnvalue (`self.GetFocusedActorDetails`))
  (bind (_actorname _interacttype) (break `FocusedActorDetails` _returnvalue))
  (`KismetSystemLibrary.PrintString` (`KismetStringLibrary.Concat_StrStr` "ActorName: " _actorname ", Type: " (`|GetEnumeratorNameAsString` _interacttype) ", ")))

(event `IA_Test Method`
  (`self.Sample_Server method`))

(event `Sample_Server method`
  (`self.Sample_Multiclient Method`))

(event `Sample Client Method`
  (`KismetSystemLibrary.PrintString` "Client Sample Triggered")
  (`self.SetMesh` :!label _label))

(event `Key|One`
  (params (Key :type "Key Structure"))
  (:`Released`
    (`self.IA_Test Method`)))

(event `Sample_Multiclient Method`
  (`KismetSystemLibrary.PrintString` "Multiclient Sample Triggered")
  (goto _label))

(fn `OnRep_PlayerDetails`
  (bind _asplayer_ui (cast `/Game/UI/PlayerUI` (`WidgetComponent.GetWidget` (`self.mOverlayWidget`))))
  (`/Game/UI/PlayerUI.UpdateVals` :`self` _asplayer_ui))

(fn `SetMesh`
  (locals (M1 :type "SkeletalMesh Object Reference" :default "/Script/Engine.SkeletalMesh'/Game/__ExternalAssets/Elite_Soldiers/Mesh/Full_Mesh/SK_Elite_Soldier_Full_03.SK_Elite_Soldier_Full_03'") (M2 :type "SkeletalMesh Object Reference" :default "/Script/Engine.SkeletalMesh'/Game/__ExternalAssets/Elite_Soldiers/Mesh_UE5/Full/SKM_Elite_Soldier_Full_04.SKM_Elite_Soldier_Full_04'"))
  (if (== (`SkeletalMeshComponent.GetSkeletalMeshAsset` (`self.Mesh`)) (`local.M1`))
    (`SkeletalMeshComponent.SetSkeletalMeshAsset` (`self.Mesh`) (`local.M2`))
    (else
      (`SkeletalMeshComponent.SetSkeletalMeshAsset` (`self.Mesh`) (`local.M1`)))))

(fn `UserConstructionScript`)