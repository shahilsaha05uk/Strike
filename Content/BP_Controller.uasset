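; Player controller for a networked Terrorist vs Counter-Terrorist shooter, handling menu, spawning, HUD, team scores and weapon purchases.
; The server spawns and possesses the character's pawn, multicast sets its team, and client events build the widgets.
; On death it destroys the pawn, asks BP_GameModeLevel1 for a decision, then requests a new player after a delay.
; The Counter-Terrorist score update on possession is unwired, so only the Terrorist score initialises.
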(event `ControllerInterface.RestartPlayer`
  (set `self.hasRestarted?` true)
  (`ControllerInterface.PawnSetup` (`self.Character Details`)))

(event `self.BlueprintClient_OnSpawn`
  (bind _returnvalue (`self.GetHUD`))
  ;[0.00344 0 0.09271] When the controller Spawns
  (`/Engine/EditorBlueprintResources/StandardMacros.IsValid` _returnvalue
    (:`Is Valid`
      (set `self.mHudRef` _returnvalue)
      (bind _returnvalue_2 (message `HUDInterface.WidgetInitialiser` _returnvalue "TEAM_MENU"))
      (set `BaseWidget.ControllerRef` self _returnvalue_2)
      (`UserWidget.AddToViewport` _returnvalue_2 0))))

(event `ServerRPC_RequestDecision`
  (params (KilledBy :type "Controller Object Reference"))
  (bind _asbp_game_mode_level_1 (cast `/Game/TEST/BP_GameModeLevel1` (`GameplayStatics.GetGameMode`)))
  (`/Game/TEST/BP_GameModeLevel1.TakeDecision` _asbp_game_mode_level_1 self KilledBy))

(event `self.BlueprintServer_SpawnPawn`
  (params (CharacterDetails :type "DA_CharacterMeshDetails Object Reference") (FindStartTransform :type "Transform Structure (by ref)"))
  ;[0.00344 0 0.09271] Spawns the Player
  (bind _output_get (set `self.Character Details` CharacterDetails))
  (bind _returnvalue (`|SpawnActorFromClass` (`DA_CharacterMeshDetails.PlayerActor` _output_get) FindStartTransform "Undefined" "MultiplyWithRoot" null null))
  (`self.Possess` _returnvalue)
  (add `self.OnPawnDead` (delegate `On PlayerDead`)))

(event `ServerRPC_RequestPlayer`
  (bind _asbp_game_mode_level_1 (cast `/Game/TEST/BP_GameModeLevel1` (`GameplayStatics.GetGameMode`)))
  (`/Game/TEST/BP_GameModeLevel1.RequestNewPlayer` _asbp_game_mode_level_1 self))

(event `On PlayerDead` :!signature `self.OnPawnDead`
  (params (InstigatedBy :type "Controller Object Reference"))
  (`|ExecutionSequence`
    (:`then_0`
      (`self.K2_DestroyActor` (`self.K2_GetPawn`)))
    (:`then_1`
      (`KismetSystemLibrary.PrintString` "Play Particles" true true (struct :`R` 1.0 :`G` 0.116176 :`A` 1.0) 3.0))
    (:`then_2`
      (`self.ServerRPC_RequestDecision` InstigatedBy))
    (:`then_3`
      (`KismetSystemLibrary.Delay` 3.0)
      (`self.ServerRPC_RequestPlayer`))))

(event `self.BlueprintMulticast_PawnSetup`
  (params (CharacterDetails :type "DA_CharacterMeshDetails Object Reference"))
  (bind _playerteam (`DA_CharacterMeshDetails.PlayerTeam` CharacterDetails))
  (message `PlayerStateInterface.InitialisePlayerState` (`self.PlayerState`) _playerteam)
  (`ControllerInterface.SetPlayerTeam` _playerteam))

(event `self.BlueprintClient_PostPossessed`
  (bind _returnvalue (message `HUDInterface.OnPawnSpawn` (`self.GetHUD`)))
  (bind _returnvalue_2 (message `PlayerStateInterface.GetPlayerDetails` (`self.PlayerState`)))
  (`PlayerHUD.UpdateHUD` _returnvalue _returnvalue_2)
  (bind _asbp_game_state (cast `/Game/BP_GameState` (`GameplayStatics.GetGameState`)))
  (bind (_terrorist _counterterrorist) (`/Game/BP_GameState.GetGameScores` _asbp_game_state))
  (`PlayerHUD.UpdateScore` _returnvalue _terrorist "TERRORIST")
  (`UserWidget.AddToViewport` _returnvalue 0))

(event `ControllerInterface.UpdateScoreboard`
  (params (Value :type Integer) (Team :type "ETeam Enum" :default "NONE"))
  (bind _returnvalue (message `HUDInterface.GetWidget` (`self.GetHUD`) "PLAYER_HUD"))
  (bind _asw_player_hud (cast `/Game/UI/W_PlayerHUD` _returnvalue))
  (`/Game/UI/W_PlayerHUD.UpdateScore` _asw_player_hud Value Team))

(fn `DestroyWidget`
  (bind _tmpwidget (`self.tmpWidget`))
  (`/Engine/EditorBlueprintResources/StandardMacros.IsValid` _tmpwidget
    (:`Is Valid`
      (`Widget.RemoveFromParent` _tmpwidget))))

(fn `UserConstructionScript`)