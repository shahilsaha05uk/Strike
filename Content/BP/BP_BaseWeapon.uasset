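; Base weapon Blueprint for an equippable, replicated gun that fires projectiles and handles equipping.
; Fire and StopFire route through server calls to multicasts; multicast fire re-arms a one-shot timer for automatic fire until stop clears it.
; Each shot attaches a muzzle effect, plays a sound and spawns BP_Bullet.
; A debug-drawn trace from the owner's camera, obtained through PlayerInputInterface, has an unused result, and GunEffect is empty.
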(event `self.Fire`
  ;[0 0 0] Fire/StopFire
  ;;[1 0.8813 0] Server Call for Fire/Stop Fire
  (`self.Server_Fire`))

(event `self.Blueprint_Multicast_Fire`
  (bind (_location _rotation) (`self.GetOwnerCameraWorldLocAndRot`))
  (bind _returnvalue (`KismetMathLibrary.GetForwardVector` _rotation))
  ;[0 0 0] Fire/StopFire
  ;;[0.1008 1 0] Firing/StopFiring
  (bind _returnvalue_2 (`KismetSystemLibrary.K2_SetTimerDelegate` (delegate `self.Blueprint_Multicast_Fire`) (`self.BulletSpeed`)))
  (set `self.TimerHandle` _returnvalue_2)
  (bind _outhit (`KismetSystemLibrary.LineTraceSingle` :`Start` (+ _location _returnvalue) :`End` (+ _location (* _returnvalue (`self.Range`))) :`TraceChannel` "TraceTypeQuery3" :`DrawDebugType` "ForDuration"))
  (`GameplayStatics.SpawnEmitterAttached` "/Game/StarterContent/Particles/P_Explosion.P_Explosion" (`self.mProjectileSpawnLocation`) "None" (0.0 0.0 0.0) (struct) (0.2 0.2 0.2) "SnapToTargetIncludingScale" true "AutoRelease")
  (`self.PlayWeaponSound`)
  (`|SpawnActorFromClass` "/Game/BP/BP_Bullet.BP_Bullet_C" (`SceneComponent.K2_GetComponentToWorld` (`self.mProjectileSpawnLocation`)) "Undefined" "MultiplyWithRoot" null null))

(event `self.StopFire`
  ;[0 0 0] Fire/StopFire
  ;;[1 0.8813 0] Server Call for Fire/Stop Fire
  (`self.Server_StopFire`))

(event `self.Blueprint_Server_Fire`
  ;[0 0 0] Fire/StopFire
  ;;[0 0.03636 1] Blueprint Server Fire/Stop Fire
  (`self.Multicast_Fire`))

(event `self.Blueprint_Multicast_StopFire`
  ;[0 0 0] Fire/StopFire
  ;;[0.1008 1 0] Firing/StopFiring
  (`KismetSystemLibrary.K2_ClearAndInvalidateTimerHandle` (`self.TimerHandle`)))

(event `self.Blueprint_ServerStopFire`
  ;[0 0 0] Fire/StopFire
  ;;[0 0.03636 1] Blueprint Server Fire/Stop Fire
  (`self.Multicast_StopFire`))

(event `self.PlayWeaponSound`
  ;[1 1 1] Sound
  (`GameplayStatics.PlaySoundAtLocation` (`self.Sound`) (`SceneComponent.RelativeLocation` (`self.mProjectileSpawnLocation`)) (struct) 1.0 1.0 0.0 null null null null))

(event `EquippableInterface.OnEquip`
  (`KismetSystemLibrary.PrintString` (`KismetStringLibrary.Concat_StrStr` "Weapon Equipped: " (`self.WeaponName`)))
  (set `PrimitiveComponent.bGenerateOverlapEvents` false (`self.mCollisionComponent`))
  (`WidgetComponent.SetDrawAtDesiredSize` (`self.mUIComponent`) false))

(fn `GetInteractType`
  (returns (ReturnValue :type Byte))
  (return 0))

(fn `GetOwnerCameraWorldLocAndRot`
  (returns (Location :type "Vector Structure") (Rotation :type "Rotator Structure"))
  (if (`KismetSystemLibrary.DoesImplementInterface` (`self.mOwnerRef`) "/Script/MultiplayerProject.PlayerInputInterface")
    (bind _returnvalue (message `PlayerInputInterface.GetFollowCamera` (`self.mOwnerRef`)))
    (return (`SceneComponent.K2_GetComponentLocation` _returnvalue) (`SceneComponent.K2_GetComponentRotation` _returnvalue))))

(fn `GunEffect`
  (params (DoesHit :type Boolean) (ImpactPoint :type "Vector Structure") (TraceEnd :type "Vector Structure")))

(fn `UserConstructionScript`)