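; Team flag actor for a capture-the-flag mode that detects pickup range and scoring at bases.
; Sphere overlap stores the flag reference on the entering player.
; Box overlap with another team's base detaches and resets the flag, then a server RPC reports the capture to BP_GameMode.
; Pickup calls the parent logic, then compares teams only to print a retrieve or capture debug message.
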(event `self.OnBoxColliderBeginOverlap`
  (params (OverlappedComponent :type "PrimitiveComponent Object Reference") (OtherActor :type "Actor Object Reference") (OtherComp :type "PrimitiveComponent Object Reference") (OtherBodyIndex :type Integer) (bFromSweep :type Boolean) (SweepResult :type "HitResult Structure (by ref)"))
  (if (`KismetSystemLibrary.DoesImplementInterface` OtherActor "/Game/BP/Interfaces/BI_TeamBaseInterface.BI_TeamBaseInterface_C")
    (bind _team (message `/Game/BP/Interfaces/BI_TeamBaseInterface.GetTeam` OtherActor))
    (if (`|EnumInequality` _team (`self.mFlagTeam`))
      (`KismetSystemLibrary.PrintString` (`KismetStringLibrary.Concat_StrStr` "Points to : " (`|GetEnumeratorNameAsString` _team)))
      (`SceneComponent.K2_DetachFromComponent` (`self.mRoot`) "KeepWorld" "KeepRelative" "KeepWorld" true)
      (`self.ResetFlag`)
      (`self.ServerRPC_UpdateRound` (`self.mPlayerStateRef`) self))))

(event `self.OnBoxColliderEndOverlap`
  (params (OverlappedComponent :type "PrimitiveComponent Object Reference") (OtherActor :type "Actor Object Reference") (OtherComp :type "PrimitiveComponent Object Reference") (OtherBodyIndex :type Integer)))

(event `ServerRPC_UpdateRound`
  (params (PlayerStateRef :type "PlayerState Object Reference") (FlagRef :type "Actor Object Reference"))
  (bind _asbp_game_mode (cast `/Game/BP/BP_GameMode` (`GameplayStatics.GetGameMode`)))
  (`/Game/BP/BP_GameMode.OnFlagCaptured` _asbp_game_mode PlayerStateRef FlagRef))

(event `self.OnSphereColliderBeginOverlap`
  (params (OverlappedComponent :type "PrimitiveComponent Object Reference") (OtherActor :type "Actor Object Reference") (OtherComp :type "PrimitiveComponent Object Reference") (OtherBodyIndex :type Integer) (bFromSweep :type Boolean) (SweepResult :type "HitResult Structure (by ref)"))
  (if (`KismetSystemLibrary.DoesImplementInterface` OtherActor "/Script/MultiplayerProject.PlayerInterface")
    (bind _asbp_parent_player (cast `/Game/BP/BP_ParentPlayer` OtherActor))
    (set `PlayerCharacter.mFlagRef` self _asbp_parent_player)
    (`KismetSystemLibrary.PrintString` "Player entered the Range")))

(event `self.OnSphereColliderEndOverlap`
  (params (OverlappedComponent :type "PrimitiveComponent Object Reference") (OtherActor :type "Actor Object Reference") (OtherComp :type "PrimitiveComponent Object Reference") (OtherBodyIndex :type Integer)))

(event `self.OnPickedUp`
  (params (PlayerState :type "PlayerState Object Reference"))
  (`parent.OnPickedUp` PlayerState)
  (bind _returnvalue (message `PlayerStateInterface.GetPlayerDetails` PlayerState))
  (if (`|EnumEquality` (`self.mFlagTeam`) (`.Team` (break `PlayerDetails` _returnvalue)))
    (`KismetSystemLibrary.PrintString` "Retrieve" true true (struct :`A` 1.0) 100.0)
    (else
      (`KismetSystemLibrary.PrintString` "Capture" true true (struct :`A` 1.0) 100.0))))

(fn `UserConstructionScript`)