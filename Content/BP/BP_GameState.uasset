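; Game state for a Terrorist versus Counter-Terrorist match, tracking team scores and the winner.
; On BeginPlay, a server RPC reads the host's target score from the game instance and multicasts it.
; Score RepNotifies update scoreboards through each player's controller interface.
; ProcessScores sets the winner when a score exceeds the target, and its RepNotify sends session-end results to every PlayerState via a server RPC.
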(event `MulticastRPC_GetTarget`
  (params (TargetScore :type Integer))
  ;[0 0 0] Gettting the Target Score Set by the Host
  (set `self.TargetScore` TargetScore))

(event `self.ReceiveBeginPlay`
  ;[0 0 0] Gettting the Target Score Set by the Host
  (`self.ServerRPC_GetTarget`))

(event `AddPointsToTeam`
  (params (Team :type "ETeam Enum" :default "NONE") (PointsToAdd :type Integer))
  ;[0 0 0] Adding Points to the Team
  (switch `ETeam` Team
    (:`TERRORIST`
      (set `self.TerroristScore` (+ (`self.TerroristScore`) PointsToAdd)))
    (:`COUNTER_TERRORIST`
      (set `self.CounterTerroristScore` (+ (`self.CounterTerroristScore`) PointsToAdd)))))

(event `ServerRPC_GetTarget`
  ;[0 0 0] Gettting the Target Score Set by the Host
  (bind _returnvalue (message `GameInstanceInterface.GetMatchDetails` (`GameplayStatics.GetGameInstance`)))
  (`self.MulticastRPC_GetTarget` (`.TargetScore` (break `MatchDetails` _returnvalue))))

(event `ServerRPC_CallSessionEnd`
  (params (WinningTeam :type "ETeam Enum" :default "NONE"))
  ;[0 0 0] When the Session Ends
  (for _array_element (`self.PlayerArray`)
    (message `PlayerStateInterface.OnSessionEnd` _array_element WinningTeam (`self.TerroristScore`) (`self.CounterTerroristScore`))))

(event `ProcessScores`
  ;[0 0 0] Checks for the Team Win!!
  (if (> (`self.CounterTerroristScore`) (`self.TargetScore`))
    (set `self.WinningTeam` "COUNTER_TERRORIST")
    (elif (> (`self.TerroristScore`) (`self.TargetScore`))
      (set `self.WinningTeam` "TERRORIST"))))

(fn `GetGameScores`
  (returns (Terrorist :type Integer) (CounterTerrorist :type Integer))
  (return (`self.TerroristScore`) (`self.CounterTerroristScore`)))

(fn `OnRep_CounterTerroristScore`
  (`self.UpdatePlayerHUDScoreBoard` "COUNTER_TERRORIST"))

(fn `OnRep_TerroristScore`
  (`self.UpdatePlayerHUDScoreBoard` "TERRORIST"))

(fn `OnRep_WinningTeam`
  (if (`|EnumInequality` (`self.WinningTeam`) "NONE")
    (`self.ServerRPC_CallSessionEnd` (`self.WinningTeam`))))

(fn `UpdatePlayerHUDScoreBoard`
  (params (Team :type "ETeam Enum" :default "NONE"))
  (locals (Score :type Integer))
  (switch `ETeam` Team
    (:`TERRORIST`
      (set `local.Score` (`self.TerroristScore`))
      (for _array_element (`self.PlayerArray`)
        (bind _returnvalue (`PlayerState.GetPawn` _array_element))
        (`/Engine/EditorBlueprintResources/StandardMacros.IsValid` _returnvalue
          (:`Is Valid`
            (bind _returnvalue_2 (`Pawn.GetController` _returnvalue))
            (if (`KismetSystemLibrary.DoesImplementInterface` _returnvalue_2 "/Script/MultiplayerProject.ControllerInterface")
              (message `ControllerInterface.UpdatePlayerHUDDetails` _returnvalue_2 "T_SCORE_Val" (`KismetStringLibrary.Conv_IntToString` (`local.Score`))))))))
    (:`COUNTER_TERRORIST`
      (set `local.Score` (`self.CounterTerroristScore`))
      (for _array_element_2 (`self.PlayerArray`)
        (bind _returnvalue_3 (`PlayerState.GetPawn` _array_element_2))
        (`/Engine/EditorBlueprintResources/StandardMacros.IsValid` _returnvalue_3
          (:`Is Valid`
            (bind _returnvalue_4 (`Pawn.GetController` _returnvalue_3))
            (if (`KismetSystemLibrary.DoesImplementInterface` _returnvalue_4 "/Script/MultiplayerProject.ControllerInterface")
              (message `ControllerInterface.UpdatePlayerHUDDetails` _returnvalue_4 "CT_SCORE_Val" (`KismetStringLibrary.Conv_IntToString` (`local.Score`))))))))))

(fn `UserConstructionScript`)