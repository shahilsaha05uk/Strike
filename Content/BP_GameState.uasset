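; Game state for a Terrorist vs Counter-Terrorist team match that tracks both team scores.
; AddPointsToTeam increments a team's score, and GetGameScores exposes both.
; Each score's RepNotify loops PlayerArray and pushes the new value to valid pawns' controllers through ControllerInterface to update HUD scoreboards.
; On the session-end event, it compares scores and prints the winner or a tie.
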(event `self.ReceiveBeginPlay`
  (add `self.OnSessionEndSignature` (delegate `OnSessionEnd`)))

(event `OnSessionEnd`
  (if (== (`self.TerroristScore`) (`self.CounterTerroristScore`))
    (`KismetSystemLibrary.PrintString` "Its a Tie!!")
    (elif (> (`self.TerroristScore`) (`self.CounterTerroristScore`))
      (`KismetSystemLibrary.PrintString` "Terrorist Wins")
      (else
        (`KismetSystemLibrary.PrintString` "Counter Terrorist Wins")))))

(event `AddPointsToTeam`
  (params (Team :type "ETeam Enum" :default "NONE"))
  (`KismetSystemLibrary.PrintString` (`KismetStringLibrary.Concat_StrStr` "Add points to: " (`|GetEnumeratorNameAsString` Team)) true true (struct :`A` 1.0) 10.0)
  (switch `ETeam` Team
    (:`TERRORIST`
      (bind _result (`/Engine/EditorBlueprintResources/StandardMacros.IncrementInt` (`self.TerroristScore`))
        (:`  `
          (set `self.TerroristScore` _result))))
    (:`COUNTER_TERRORIST`
      (bind _result_2 (`/Engine/EditorBlueprintResources/StandardMacros.IncrementInt` (`self.CounterTerroristScore`))
        (:`  `
          (set `self.CounterTerroristScore` _result_2))))))

(fn `GetGameScores`
  (returns (Terrorist :type Integer) (CounterTerrorist :type Integer))
  (return (`self.TerroristScore`) (`self.CounterTerroristScore`)))

(fn `OnRep_CounterTerroristScore`
  (`self.UpdatePlayerHUDScoreBoard` "COUNTER_TERRORIST"))

(fn `OnRep_TerroristScore`
  (`self.UpdatePlayerHUDScoreBoard` "TERRORIST"))

(fn `UpdatePlayerHUDScoreBoard`
  (params (Team :type "ETeam Enum" :default "NONE"))
  (switch `ETeam` Team
    (:`TERRORIST`
      (for _array_element (`self.PlayerArray`)
        (bind _returnvalue (`PlayerState.GetPawn` _array_element))
        (`/Engine/EditorBlueprintResources/StandardMacros.IsValid` _returnvalue
          (:`Is Valid`
            (bind _returnvalue_2 (`Pawn.GetController` _returnvalue))
            (if (`KismetSystemLibrary.DoesImplementInterface` _returnvalue_2 "/Script/MultiplayerProject.ControllerInterface")
              (message `ControllerInterface.UpdateScoreboard` _returnvalue_2 (`self.TerroristScore`) Team))))))
    (:`COUNTER_TERRORIST`
      (for _array_element_2 (`self.PlayerArray`)
        (bind _returnvalue_3 (`PlayerState.GetPawn` _array_element_2))
        (`/Engine/EditorBlueprintResources/StandardMacros.IsValid` _returnvalue_3
          (:`Is Valid`
            (bind _returnvalue_4 (`Pawn.GetController` _returnvalue_3))
            (if (`KismetSystemLibrary.DoesImplementInterface` _returnvalue_4 "/Script/MultiplayerProject.ControllerInterface")
              (message `ControllerInterface.UpdateScoreboard` _returnvalue_4 (`self.CounterTerroristScore`) Team))))))))

(fn `UserConstructionScript`)