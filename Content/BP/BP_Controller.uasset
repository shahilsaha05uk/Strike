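; BP_Controller is the player controller for a Terrorist versus Counter-Terrorist match, linking each player to the game mode, HUD and results screen.
; On possession it fills the spawn HUD with player details, target and team scores.
; It forwards kill/capture decisions and respawn requests to BP_GameMode, relays health and HUD updates, and deducts weapon costs from player-state money.
; On session end it shows the result widget, pauses and unpossesses.
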(event `self.BlueprintClient_PostPossessed`
  (params (PlayerDetails :type "PlayerDetails Structure") (MatchDetails :type "MatchDetails Structure"))
  ;[0 0 0] When the Client Has been Possessed
  (bind _returnvalue (message `HUDInterface.OnPawnSpawn` (`self.GetHUD`)))
  (`PlayerHUDInterface.UpdateTarget` _returnvalue (`.TargetScore` (break `MatchDetails` MatchDetails)))
  (message `PlayerHUDInterface.UpdateHUD` _returnvalue PlayerDetails)
  (message `PlayerHUDInterface.UpdateHUD` _returnvalue PlayerDetails)
  (bind _asbp_game_state (cast `/Game/BP/BP_GameState` (`GameplayStatics.GetGameState`)))
  (bind (_terrorist _counterterrorist) (`/Game/BP/BP_GameState.GetGameScores` _asbp_game_state))
  (`|ExecutionSequence`
    (:`then_0`
      (message `PlayerHUDInterface.UpdateScore` _returnvalue _terrorist "TERRORIST"))
    (:`then_1`
      (message `PlayerHUDInterface.UpdateScore` _returnvalue _counterterrorist "COUNTER_TERRORIST")
      (`UserWidget.AddToViewport` _returnvalue 0))))

(event `self.RequestNewPlayer`
  ;[0 0 0] Request for a new Player after they die
  (bind _asbp_game_mode (cast `/Game/BP/BP_GameMode` (`GameplayStatics.GetGameMode`)))
  (`/Game/BP/BP_GameMode.RequestNewPlayer` _asbp_game_mode self))

(event `self.BlueprintServer_RequestGameModeDecision`
  (params (InstigatorController :type "Controller Object Reference"))
  ;[0 0 0] GameMode to take Decision on Kill/Capture
  (bind _asbp_game_mode (cast `/Game/BP/BP_GameMode` (`GameplayStatics.GetGameMode`)))
  (`/Game/BP/BP_GameMode.TakeDecision` _asbp_game_mode self InstigatorController))

(event `ControllerInterface.OnSessionEnd`
  (params (WinningTeam :type "ETeam Enum" :default "NONE") (TScore :type Integer) (CTScore :type Integer))
  ;[0 0 0] When the Session Ends
  (bind _returnvalue (`|CreateWidget` "/Game/UI/W_ResultWidget.W_ResultWidget_C" null null null))
  (`/Game/UI/W_ResultWidget.Update_Texts` _returnvalue WinningTeam TScore CTScore)
  (`UserWidget.AddToViewport` _returnvalue 0)
  (`GameplayStatics.SetGamePaused` true)
  (set `self.bShowMouseCursor` true)
  (`self.UnPossess`))

(event `AddHealth`
  (params (Value :type "Float (single-precision)"))
  (message `PlayerStateInterface.UpdateHealth` (`self.PlayerState`) Value))

(event `ControllerInterface.UpdatePlayerHUDDetails`
  (params (ValueType :type "EHUDValue Enum" :default "AMMO_Val") (Value :type String))
  (bind _returnvalue (message `HUDInterface.GetWidget` (`self.GetHUD`) "PLAYER_HUD"))
  (bind _asw_player_hud (cast `/Game/UI/W_PlayerHUD` _returnvalue))
  (`/Game/UI/W_PlayerHUD.UpdateDetails` _asw_player_hud ValueType Value))

(fn `UserConstructionScript`)