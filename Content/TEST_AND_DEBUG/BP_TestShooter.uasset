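; BP_TestShooter is a debug actor that periodically fires a line trace and reports what it detects.
; BeginPlay calls ShootLaser immediately and on a looping timer.
; Each shot traces from the Arrow component, ignoring itself and its owner, draws a persistent debug line and prints the hit actor's name.
; The trace end multiplies the sum of location and forward vector by TraceRange, rather than scaling only the direction.
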(event `self.ReceiveBeginPlay`
  (`KismetSystemLibrary.K2_SetTimerDelegate` (delegate `ShootLaser`) 2.0 true)
  (`self.ShootLaser`))

(event `ShootLaser`
  (bind _arrow (`self.Arrow`))
  (bind _returnvalue (`SceneComponent.K2_GetComponentLocation` _arrow))
  (bind _outhit (`KismetSystemLibrary.LineTraceSingle` _returnvalue (* (+ _returnvalue (`SceneComponent.GetForwardVector` _arrow)) (`self.TraceRange`)) "TraceTypeQuery3" false (`|MakeArray` (`self.GetOwner`) self :!type "Actor Object Reference") "Persistent" true (struct :`R` 0.09217 :`B` 1.0 :`A` 1.0)))
  (`KismetSystemLibrary.PrintString` (`KismetStringLibrary.Concat_StrStr` "Actor detects: " (`KismetSystemLibrary.GetDisplayName` (`.HitActor` (`GameplayStatics.BreakHitResult` _outhit))))))

(fn `UserConstructionScript`)