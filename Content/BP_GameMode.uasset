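; Game mode for a team-based flag-capture game, awarding team points for kills and enemy flag captures through BP_GameState, which then processes scores.
; It tracks joining controllers that implement ControllerInterface and forwards respawn requests to them as restart messages.
; FindPlayerStart lazily maps teams to BP_WorldBase actors, then spawns a PlayerStart at a random point within the team base's box, retrying until valid, or falls back to default selection.
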(event `self.HandleStartingNewPlayer`
  (params (NewPlayer :type "PlayerController Object Reference"))
  (`parent.HandleStartingNewPlayer` NewPlayer)
  (if (`KismetSystemLibrary.DoesImplementInterface` NewPlayer "/Script/MultiplayerProject.ControllerInterface")
    (`KismetArrayLibrary.Array_AddUnique` (`self.Controllers`) NewPlayer)
    (for _ (`self.Controllers`)
      _)))

(event `TakeDecision`
  (params (DamagedController :type "Controller Object Reference") (InstigatorController :type "Controller Object Reference"))
  (bind _asbp_game_state (cast `/Game/BP_GameState` (`GameplayStatics.GetGameState`)))
  (bind _returnvalue (message `PlayerStateInterface.GetPlayerDetails` (`Controller.PlayerState` InstigatorController)))
  (`/Game/BP_GameState.AddPointsToTeam` _asbp_game_state (`.Team` (break `PlayerDetails` _returnvalue)) (`self.PointsToAddOnKill`))
  (`/Game/BP_GameState.ProcessScores` _asbp_game_state))

(event `RequestNewPlayer`
  (params (DamagedControllerRef :type "Controller Object Reference"))
  (message `ControllerInterface.RestartPlayer` (`|GetArrayItem` (`self.Controllers`) (`self.Get Controller` DamagedControllerRef))))

(event `OnUpdateRound`
  (params (PlayerStateRef :type "PlayerState Object Reference") (FlagRef :type "Actor Object Reference"))
  (if (and (`KismetSystemLibrary.DoesImplementInterface` PlayerStateRef "/Script/MultiplayerProject.PlayerStateInterface") (`KismetSystemLibrary.DoesImplementInterface` FlagRef "/Script/MultiplayerProject.FlagInterface"))
    (bind _returnvalue (message `FlagInterface.GetFlagTeam` FlagRef))
    (bind _returnvalue_2 (message `PlayerStateInterface.GetPlayerDetails` PlayerStateRef))
    (bind (_playername _currentmoney _team) (break `PlayerDetails` _returnvalue_2))
    (if (`|EnumInequality` _team _returnvalue)
      (bind _asbp_game_state (cast `/Game/BP_GameState` (`GameplayStatics.GetGameState`)))
      (`/Game/BP_GameState.AddPointsToTeam` _asbp_game_state _team (`self.PointsToAddOnCapture`))
      (`/Game/BP_GameState.ProcessScores` _asbp_game_state))))

(event `self.K2_PostLogin`
  (params (NewPlayer :type "PlayerController Object Reference")))

(fn `FindPlayerStart`
  (params (Player :type "Controller Object Reference") (IncomingName :type String))
  (returns (ReturnValue :type "Actor Object Reference"))
  (bind _returnvalue (message `PlayerStateInterface.GetPlayerDetails` (`Controller.PlayerState` Player)))
  (bind ((`Team` _team)) (break `PlayerDetails` _returnvalue))
  (if (`.ReturnValue` (`BlueprintMapLibrary.Map_Find` (`self.GetTeamBases`) _team))
    (bind _value (`self.SpawnPlayerStart` _team :!label _label))
    (`/Engine/EditorBlueprintResources/StandardMacros.IsValid` _value
      (:`Is Valid`
        (return _value))
      (:`Is Not Valid`
        (goto _label)))
    (else
      (bind _returnvalue_2 (`parent.FindPlayerStart` (`local.Player`) (`local.IncomingName`)))
      (return _returnvalue_2))))

(fn `Get Controller`
  (params (ControllerRef :type "Controller Object Reference"))
  (returns (ControllerID :type Integer))
  (bind _asplayer_controller (cast `PlayerController` ControllerRef))
  (bind _returnvalue (`KismetArrayLibrary.Array_Find` (`self.Controllers`) _asplayer_controller))
  (if (!= _returnvalue -1)
    (return _returnvalue)
    (else
      (`KismetSystemLibrary.PrintString` "Controller Is NOT VALID" true true (struct :`R` 1.0 :`G` 0.030432 :`A` 1.0) 10.0))))

(fn `GetTeamBases`
  (returns (TeamBases :type "Map of ETeam Enum to /Game/BP/BP_WorldBase Object Reference"))
  (bind _teambases (`self.TeamBases`))
  (if (`BlueprintMapLibrary.Map_IsEmpty` _teambases)
    (bind _outactors (`GameplayStatics.GetAllActorsOfClass` "/Game/BP/BP_WorldBase.BP_WorldBase_C"))
    (for _array_element _outactors
      (`BlueprintMapLibrary.Map_Add` (`self.TeamBases`) (`/Game/BP/BP_WorldBase.TeamBase` _array_element) _array_element))
    (return (`self.TeamBases`))
    (else
      (return _teambases))))

(fn `OnRep_Controllers`)

(fn `SpawnPlayerStart`
  (params (Team :type "ETeam Enum" :default "NONE"))
  (returns (Value :type "PlayerStart Object Reference"))
  (bind _keys (`BlueprintMapLibrary.Map_Keys` (`self.TeamBases`)))
  (bind _returnvalue (`KismetArrayLibrary.Array_Find` _keys Team))
  (if (!= _returnvalue -1)
    (bind _values (`BlueprintMapLibrary.Map_Values` (`self.TeamBases`)))
    (bind (_origin _boxextent) (`KismetSystemLibrary.GetComponentBounds` (`/Game/BP/BP_WorldBase.Box` (`|GetArrayItem` _values _returnvalue))))
    (bind (_returnvalue_x _returnvalue_y) (`KismetMathLibrary.BreakVector` (`KismetMathLibrary.RandomPointInBoundingBox` _origin _boxextent)))
    (bind _returnvalue_2 (`|SpawnActorFromClass` "/Script/Engine.PlayerStart" (`KismetMathLibrary.MakeTransform` (`KismetMathLibrary.MakeVector` _returnvalue_x _returnvalue_y 200.0)) "Undefined" "MultiplyWithRoot" null null))
    (return _returnvalue_2)))

(fn `UserConstructionScript`)